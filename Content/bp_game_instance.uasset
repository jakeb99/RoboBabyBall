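; Game instance Blueprint that keeps the running player score and determines which level follows the current one.
; A custom event adds the temporary score to the total.
; NextLevelFromCurrent looks up the current level's index in the Levels map, increments it and returns the key at that position, relying on key order.
; A hardcoded final index returns the main menu instead.
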(event Custom|CalculateTotalScore
  ;[1 1 1] Calculate total score
  (Variables|Default|SettotalPlayerScore (+ (Variables|Default|GettotalPlayerScore) (Variables|Default|GettempPlayerScore))))

(fn NextLevelfromCurrent
  (bind _levels (Variables|Default|GetLevels))
  (bind _returnvalue (Game|GetCurrentLevelName true))
  (bind _result (Math|Integer|IncrementInt (.Value (Utilities|Map|Find _levels _returnvalue)))
    (:%20%20
      (bind _output_get (Variables|Default|SetnextLevelIndex _result))
      (Development|PrintString (Utilities|String|ToString(Integer) _output_get))
      (bind _keys (Utilities|Map|Keys _levels))
      (if (== _output_get 8)
        (return "MainMenu")
        (else
          (bind (_array_element _array_index) (Utilities|Array|ForEachLoopwithBreak _keys :!label _label)
            (:LoopBody
              (if (== _array_index (Variables|Default|GetnextLevelIndex))
                (Variables|Default|SetnextLevel _array_element)
                (goto _label Break)))
            (:Completed
              (Variables|Default|SetnextLevelIndex 0)
              (return (Variables|Default|GetnextLevel)))))))))