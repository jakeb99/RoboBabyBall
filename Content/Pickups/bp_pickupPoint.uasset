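; Score pickup Blueprint that spins in place and awards a point when the player ball touches it.
; Tick applies a local rotation from the roll, pitch and yaw speed variables, scaled by delta time.
; On overlap with bp_playerBall it plays a blip sound at the ball's location, destroys itself, then adds to the score through primary_gamemode.
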(event EventBeginPlay)

(event EventTick
  (params (DeltaSeconds :type Float%20%28single-precision%29))
  ;[1 1 1] Rotates the pickup
  (Transformation|AddActorLocalRotation (* (Math|Rotator|MakeRotator (Variables|Default|Getroll%20speed) (Variables|Default|Getpitch%20speed) (Variables|Default|Getyaw%20speed)) DeltaSeconds) false false))

(event Collision|EventActorBeginOverlap
  (params (OtherActor :type Actor%20Object%20Reference))
  ;[1 1 1] Destroy pick when player touches it and add score and play sound
  (bind _asbp_player_ball (Utilities|Casting|CastTobp_playerBall OtherActor))
  (Audio|PlaySoundatLocation "/Game/Audio/blip-131856.blip-131856" (Transformation|GetActorLocation _asbp_player_ball) "0, 0, 0" 1.0 1.0 0.0 0 0 0)
  (Actor|DestroyActor)
  (bind _asprimary_gamemode (Utilities|Casting|CastToprimary_gamemode (Game|GetGameMode)))
  (Default|AddScore _asprimary_gamemode 1))

(fn ConstructionScript)