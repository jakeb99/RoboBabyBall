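; Checkpoint pickup that sets a new spawn location when reached by the player ball.
; A cube rotates every tick at configurable roll, pitch and yaw speeds.
; Box overlap passes the checkpoint to the game mode via a message, without checking what overlapped.
; Player-ball overlap plays a sound, destroys the box and cube but keeps the actor, and has primary_gamemode show checkpoint text.
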(event OnComponentBeginOverlap(Box)
  (params (OverlappedComponent :type Primitive%20Component%20Object%20Reference) (OtherActor :type Actor%20Object%20Reference) (OtherComp :type Primitive%20Component%20Object%20Reference) (OtherBodyIndex :type Integer) (bFromSweep :type Boolean) (SweepResult :type Hit%20Result%20Structure%20%28by%20ref%29))
  ;[1 1 1] Update spawn location
  (Class|BpiUpdateSpawnLocation|UpdateSpawnLocation(Message) (Game|GetGameMode) self))

(event EventTick
  (params (DeltaSeconds :type Float%20%28single-precision%29))
  ;[1 1 1] Rotates the cube
  (Transformation|AddActorLocalRotation (* (Math|Rotator|MakeRotator (Variables|Default|Getroll%20speed) (Variables|Default|Getpitch%20speed) (Variables|Default|Getyaw%20speed)) DeltaSeconds) false false))

(event Collision|EventActorBeginOverlap
  (params (OtherActor :type Actor%20Object%20Reference))
  ;[1 1 1] Destroy checkpoint when player touches and display message
  (bind _asbp_player_ball (Utilities|Casting|CastTobp_playerBall OtherActor))
  (Audio|PlaySoundatLocation "/Game/Audio/checkpoint.checkpoint" (Transformation|GetActorLocation _asbp_player_ball) "0, 0, 0" 1.0 1.0 0.0 0 0 0)
  (Components|DestroyComponent (Variables|Default|GetBox))
  (Components|DestroyComponent (Variables|Default|GetCube))
  (bind _asprimary_gamemode (Utilities|Casting|CastToprimary_gamemode (Game|GetGameMode)))
  (Default|ShowCheckpointText _asprimary_gamemode))

(fn ConstructionScript)